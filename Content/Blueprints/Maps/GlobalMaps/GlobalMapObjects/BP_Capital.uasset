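; BP_Capital is a global map object representing a named capital that players can approach and enter.
; Overlapping its contact box makes the locally controlled Map_PlayerPawn spawn a text-render announcement of the capital name via client events, destroyed on exit.
; Overlapping the capital mesh passes a Russian "press F to enter" prompt and the capital name to GlobalMap_Character's connection data for server entry, cleared on exit.
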(event OnComponentBeginOverlap(PlayerContactBox)
  (params (OverlappedComponent :type Primitive%20Component%20Object%20Reference) (OtherActor :type Actor%20Object%20Reference) (OtherComp :type Primitive%20Component%20Object%20Reference) (OtherBodyIndex :type Integer) (bFromSweep :type Boolean) (SweepResult :type Hit%20Result%20Structure%20%28by%20ref%29))
  ;[1 1 1] On player character enteres the given area - show an info text to him
  (bind _asmap_player_pawn (Utilities|Casting|CastToMap_PlayerPawn OtherActor))
  (if (Pawn|IsLocallyControlled _asmap_player_pawn)
    (CallFunction|Client||SpawnAnnouncementText _asmap_player_pawn)))

(event OnComponentEndOverlap(PlayerContactBox)
  (params (OverlappedComponent :type Primitive%20Component%20Object%20Reference) (OtherActor :type Actor%20Object%20Reference) (OtherComp :type Primitive%20Component%20Object%20Reference) (OtherBodyIndex :type Integer))
  ;[1 1 1] On player character enteres the given area - show an info text to him
  (bind _asmap_player_pawn (Utilities|Casting|CastToMap_PlayerPawn OtherActor))
  (if (Pawn|IsLocallyControlled _asmap_player_pawn)
    (CallFunction|Client||DestroyAnnouncementText)))

(event OnComponentBeginOverlap(CapitalMesh)
  (params (OverlappedComponent :type Primitive%20Component%20Object%20Reference) (OtherActor :type Actor%20Object%20Reference) (OtherComp :type Primitive%20Component%20Object%20Reference) (OtherBodyIndex :type Integer) (bFromSweep :type Boolean) (SweepResult :type Hit%20Result%20Structure%20%28by%20ref%29))
  ;[1 1 1] On character entered the capital mesh, allow him to use F key to enter its server and update info text
  (bind _asglobal_map_character (Utilities|Casting|CastToGlobalMap_Character OtherActor))
  (Default|UpdateConnectionData _asglobal_map_character (Utilities|Text|ToText(String) (Utilities|String|Append "Нажмите F, чтобы войти в" " " (Utilities|String|ToString(Name) (Variables|Default|GetCapitalName)))) (Variables|Default|GetCapitalName)))

(event OnComponentEndOverlap(CapitalMesh)
  (params (OverlappedComponent :type Primitive%20Component%20Object%20Reference) (OtherActor :type Actor%20Object%20Reference) (OtherComp :type Primitive%20Component%20Object%20Reference) (OtherBodyIndex :type Integer))
  ;[1 1 1] On character entered the capital mesh, allow him to use F key to enter its server and update info text
  (bind _asglobal_map_character (Utilities|Casting|CastToGlobalMap_Character OtherActor))
  (Default|UpdateConnectionData _asglobal_map_character "" "None"))

(event Custom|Client%20||%20SpawnAnnouncementText
  (params (ContactedCharacter :type Map%20Player%20Pawn%20Object%20Reference))
  ;[1 1 1] Spawn an destroy text on request
  (bind _returnvalue (Game|SpawnActorfromClass "/Game/Blueprints/Maps/Announcement_TextRender.Announcement_TextRender_C" (Math|Transform|MakeTransform (Transformation|GetWorldLocation (Variables|Default|GetCapitalMesh)) "0, 0, 0" "1,1,1") "Undefined" ContactedCharacter ContactedCharacter (Utilities|String|ToString(Name) (Variables|Default|GetCapitalName)) 0))
  (Variables|Default|SetSpawnedAnnouncementText _returnvalue))

(event Custom|Client%20||%20DestroyAnnouncementText
  ;[1 1 1] Spawn an destroy text on request
  (Default|ExecuteTextDestroy (Variables|Default|GetSpawnedAnnouncementText)))

(fn ConstructionScript)