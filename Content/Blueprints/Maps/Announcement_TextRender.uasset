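; Announcement text actor that shows a supplied message as world text turned toward the contacted character's camera.
; BeginPlay sets the text and triggers the appear event, which plays a timeline meant to raise and enlarge it and opens a Tick gate for the camera-facing rotation.
; The destroy event reverses the timeline, closes the gate and removes the actor after a short delay.
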(event Custom|ExecuteTextAppear
  (bind _contactedcharacter (Variables|Default|GetContactedCharacter))
  (bind _announcementtext (Variables|Default|GetAnnouncementText))
  (bind _returnvalue (Transformation|GetWorldLocation _announcementtext))
  (bind _camera (Variables|/Game/Blueprints/Maps/Map_PlayerPawn.Map_PlayerPawn_C|GetCamera _contactedcharacter))
  (bind _returnvalue_2 (Transformation|GetWorldLocation _camera))
  (bind _returnvalue_3 (- _returnvalue _returnvalue_2))
  (bind _returnvalue_4 (Math|Rotator|MakeRotfromX _returnvalue_3))
  ;[1 1 1] Execute events for appearance and destruction and text rotation towards camera on tick
  (Components|Timeline|PlayfromStart (Variables|Default|GetAnnouncementText_Timeline))
  (Utilities|FlowControl|Gate true) ; enters at Open
)

(event Custom|ExecuteTextDestroy
  (bind _contactedcharacter (Variables|Default|GetContactedCharacter))
  (bind _announcementtext (Variables|Default|GetAnnouncementText))
  (bind _returnvalue (Transformation|GetWorldLocation _announcementtext))
  (bind _camera (Variables|/Game/Blueprints/Maps/Map_PlayerPawn.Map_PlayerPawn_C|GetCamera _contactedcharacter))
  (bind _returnvalue_2 (Transformation|GetWorldLocation _camera))
  (bind _returnvalue_3 (- _returnvalue _returnvalue_2))
  (bind _returnvalue_4 (Math|Rotator|MakeRotfromX _returnvalue_3))
  ;[1 1 1] Execute events for appearance and destruction and text rotation towards camera on tick
  (Components|Timeline|ReversefromEnd (Variables|Default|GetAnnouncementText_Timeline))
  (Utilities|FlowControl|Sequence
    (:then_0
      (Utilities|FlowControl|Delay 2.0)
      (Actor|DestroyActor))
    (:then_1
      (Utilities|FlowControl|Gate true) ; enters at Close
    )))

(event EventTick
  (params (DeltaSeconds :type Float%20%28single-precision%29))
  (bind _contactedcharacter (Variables|Default|GetContactedCharacter))
  (bind _announcementtext (Variables|Default|GetAnnouncementText))
  (bind _returnvalue (Transformation|GetWorldLocation _announcementtext))
  (bind _camera (Variables|/Game/Blueprints/Maps/Map_PlayerPawn.Map_PlayerPawn_C|GetCamera _contactedcharacter))
  (bind _returnvalue_2 (Transformation|GetWorldLocation _camera))
  (bind _returnvalue_3 (- _returnvalue _returnvalue_2))
  (bind _returnvalue_4 (Math|Rotator|MakeRotfromX _returnvalue_3))
  ;[1 1 1] Execute events for appearance and destruction and text rotation towards camera on tick
  (Utilities|FlowControl|Gate true
    (:Exit
      (Transformation|SetWorldRotation (Variables|Default|GetAnnouncementText) (Math|Rotator|MakeRotator (.roll _returnvalue_4) (* (.pitch _returnvalue_4) -1.0) (- (.yaw _returnvalue_4) 1.8e+02)) false false))))

(event EventBeginPlay
  ;[1 1 1] Update text as requested and execute its appearance
  (Rendering|Components|TextRender|SetText (Variables|Default|GetAnnouncementText) (Utilities|Text|ToText(String) (Variables|Default|GetTextToShow)))
  (CallFunction|ExecuteTextAppear))

(fn ConstructionScript)