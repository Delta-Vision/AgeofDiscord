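; BP_GlobalMap_PC is the global map player controller, relaying state between the controlled character and the player's pawn.
; It stores the controlled character reference and forwards it to the pawn through message calls.
; Info text and available action name updates pass to the pawn the same way.
; A server event destroys any given actor, used to remove the controlled character on the server.
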(event Custom|Server%20||%20DestroyActor
  (params (Target :type Actor%20Object%20Reference))
  ;[1 1 1] Request server to destroy an actor
  (Actor|DestroyActor Target))

(event EventRequesttoDestroyControlledCharacteronServer
  ;[1 1 1] Request to destroy controlled character from the server
  (CallFunction|Server||DestroyActor (Variables|Default|GetControlledCharacter)))

(event EventUpdateControlledCharacterRef
  (params (Character :type Global%20Map%20Character%20Object%20Reference))
  ;[1 1 1] Update controlled character(C++)
  (Variables|Default|SetControlledCharacter Character)
  (Class|GlobalMapPawnInterface|UpdateControlledCharacterRefPawn(Message) (Pawn|GetControlledPawn) Character))

(event EventRequesttoUpdateInfoText
  (params (InfoText :type Text))
  ;[1 1 1] Request controlled pawn to update its UI text
  (Class|GlobalMapPawnInterface|RequesttoUpdateInfoTextPawn(Message) (Pawn|GetControlledPawn) InfoText))

(event EventRequesttoUpdateAvailableActionName
  (params (ActionName :type Name :default "None"))
  ;[1 1 1] Request to pdate available action for current player on any connection was occured
  (Class|GlobalMapPawnInterface|RequesttoUpdateAvailableActionNamePawn(Message) (Pawn|GetControlledPawn) ActionName))

(fn ConstructionScript)