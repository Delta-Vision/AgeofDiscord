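; Game mode for the global map that spawns each joining player's pawn and map character at the main capital.
; On BeginPlay it caches the BP_Capital actor flagged as the main location.
; On PostLogin it spawns and possesses a Map_PlayerPawn, then spawns a GlobalMap_Character owned by that controller and passes it to the controller via an interface message.
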(event EventPostLogin
  (params (NewPlayer :type Player%20Controller%20Object%20Reference))
  ;[1 1 1] On any client connected, spawn new character and allow him to possess it
  (bind _returnvalue (Game|SpawnActorfromClass "/Game/Blueprints/Maps/Map_PlayerPawn.Map_PlayerPawn_C" (Math|Transform|MakeTransform (Transformation|GetActorLocation (Variables|Default|GetCapital)) "0, 0, 0" "1,1,1") "Undefined" 0 0))
  (Pawn|Possess NewPlayer _returnvalue)
  (bind _returnvalue_2 (Game|SpawnActorfromClass "/Game/Blueprints/Maps/GlobalMaps/GlobalMap_Character/GlobalMap_Character.GlobalMap_Character_C" (Math|Transform|MakeTransform (Transformation|GetActorLocation (Variables|Default|GetCapital)) "0, 0, 0" "1,1,1") "Undefined" 0 NewPlayer 0))
  (Class|GlobalMapPCInterface|UpdateControlledCharacterRef(Message) NewPlayer _returnvalue_2))

(event EventBeginPlay
  ;[1 1 1] Find The Capital On the Map and remember its ref
  (Variables|Default|SetCapital (CallFunction|GetCapitalRef)))

(fn ConstructionScript
  (|CallParentFunction))

(fn GetCapitalRef
  (bind _outactors (Actor|GetAllActorsOfClass "/Game/Blueprints/Maps/GlobalMaps/GlobalMapObjects/BP_Capital.BP_Capital_C"))
  (for _array_element _outactors
    (if (Variables|/Game/Blueprints/Maps/GlobalMaps/GlobalMapObjects/BP_Capital.BP_Capital_C|GetbIsMainLocation _array_element)
      (return _array_element))))