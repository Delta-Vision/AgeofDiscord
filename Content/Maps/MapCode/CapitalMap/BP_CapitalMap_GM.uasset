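; BP_CapitalMap_GM is the game mode for the capital map, handling the spawning of player pawns.
; On PostLogin it spawns a BP_CapitalMap_Character at the location of the first PlayerStart found, possesses it with the new player and sets game-only input.
; GetCapitalRef is a helper that returns the first BP_Capital actor in the level.
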(event EventPostLogin
  (params (NewPlayer :type Player%20Controller%20Object%20Reference))
  ;[1 1 1] On any client connected, spawn new character and allow him to possess it
  (bind _outactors (Actor|GetAllActorsOfClass "/Script/Engine.PlayerStart"))
  (bind _returnvalue (Game|SpawnActorfromClass "/Game/Blueprints/Maps/CapitalMap/CapitalMap_Character/BP_CapitalMap_Character.BP_CapitalMap_Character_C" (Math|Transform|MakeTransform (Transformation|GetActorLocation (Utilities|Array|Get(acopy) _outactors)) "0, 0, 0" "1,1,1") "Undefined" 0 0))
  (Pawn|Possess NewPlayer _returnvalue)
  (Input|SetInputModeGameOnly NewPlayer))

(fn ConstructionScript
  (|CallParentFunction))

(fn GetCapitalRef
  (bind _outactors (Actor|GetAllActorsOfClass "/Game/Blueprints/Maps/GlobalMaps/GlobalMapObjects/BP_Capital.BP_Capital_C"))
  (return (Utilities|Array|Get(acopy) _outactors)))